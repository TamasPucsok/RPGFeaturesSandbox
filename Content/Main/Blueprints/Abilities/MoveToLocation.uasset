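; MoveToLocation is an ability actor that sends its instigator's AI controller to a target location.
; On activation it casts the instigator controller to AIController, starts a move without partial paths, and begins a looping timer.
; The timer polls move status and destroys the actor once the move goes idle; destruction sends the completed response and clears the timer.
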(event EventActivateAbility
  (params (TargetActor :type Actor%20Object%20Reference) (TargetLocation :type Vector :default "0, 0, 0"))
  (|CallParentFunction TargetActor TargetLocation)
  (bind _asaicontroller (Utilities|Casting|CastToAIController (Game|GetInstigatorController)))
  (bind _output_get (Variables|Default|SetInstigatorAI _asaicontroller))
  (AI|Navigation|MovetoLocation _output_get (Variables|Default|GetTargetLocation) 0.0 true true false true 0 false)
  (Utilities|Time|SetTimerbyFunctionName 0 "CheckEndCondition" 0.2 true))

(event EventDestroyed
  (CallFunction|SendCompletedResponse)
  (Utilities|Time|ClearTimerbyFunctionName 0 "CheckEndCondition"))

(fn ConstructionScript
  (|CallParentFunction))

(fn CheckEndCondition
  (if (Utilities|Enum|Equal(Enum) (Class|AIController|GetMoveStatus (Variables|Default|GetInstigatorAI)) "Idle")
    (Actor|DestroyActor)))