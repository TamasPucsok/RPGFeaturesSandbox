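; Actor that previews a controlled member's route through its queued commands and on to the cursor.
; It caches the command queue whenever that changes, then each tick joins synchronous navigation paths for the current move, queued moves and cursor hit.
; The joined points form a linear spline, tiled with evenly spaced spline meshes that are added or destroyed to match its length.
; All meshes are cleared when the cursor path is partial or empty.
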(event Custom|QueueChanged
  (bind _component (Class|ICommandQueue|GetCommandQueueComponent(Message) (Variables|Default|GetControlledMember)))
  (bind _output_get (Variables|Default|SetCommandQueue (Variables|/Game/Main/Blueprints/Components/CommandQueueComponent.CommandQueueComponent_C|GetExecutionQueue _component)))
  (Utilities|Array|Clear (Variables|PartialPath|GetQueuePath))
  (Variables|Default|SetIsQueueEmpty (not (> (Utilities|Array|Length _output_get) 0)))
  (if (> (Utilities|Array|Length _output_get) 0)
    (Variables|Default|SetCurrentDestination (.targetlocation (Utilities|Array|Get(acopy) _output_get)))
    (Variables|Default|SetTargetActor (.targetactor (Utilities|Array|Get(acopy) _output_get)))))

(event Custom|Init
  (params (Controller :type Player%20Controller%20Object%20Reference) (ControlledMember :type Actor%20Object%20Reference))
  (Variables|Default|SetPlayerController Controller)
  (bind _output_get (Variables|Default|SetControlledMember ControlledMember))
  (bind _component (Class|ICommandQueue|GetCommandQueueComponent(Message) _output_get))
  (EventDispatchers|BindEventtoQueueChanged _component (delegate Custom|QueueChanged))
  (CallFunction|QueueChanged))

(event EventTick
  (params (DeltaSeconds :type Float%20%28single-precision%29))
  (bind _pathpoints (PathCalculation|CalcPathtoCursor))
  (Utilities|Array|Clear (Variables|Default|GetCompletePath))
  (Variables|PartialPath|SetQueuePath (PathCalculation|CalcPlannedPath))
  (if (not (== (Utilities|Array|Length _pathpoints) 0))
    (Variables|PartialPath|SetPathToCursor _pathpoints)
    (Utilities|Array|AppendArray (Variables|Default|GetCompletePath) (PathCalculation|CalcCurrentPath))
    (Utilities|Array|AppendArray (Variables|Default|GetCompletePath) (Variables|PartialPath|GetQueuePath))
    (Utilities|Array|AppendArray (Variables|Default|GetCompletePath) (Variables|PartialPath|GetPathToCursor))
    (CallFunction|GenerateMeshes (Variables|Default|GetCompletePath))
    (else
      (CallFunction|ClearSplineMeshes))))

(fn ConstructionScript)

(fn CalcPlannedPath
  (bind _commandqueue (Variables|Default|GetCommandQueue))
  (bind _returnarray (LocalVariables|GetReturnArray))
  (LocalVariables|SetLastWaypoint (Variables|Default|GetCurrentDestination))
  (for _index (range 1 (Utilities|Array|LastIndex _commandqueue))
    (bind _returnvalue (Class|NavigationSystemV1|FindPathtoLocationSynchronously (LocalVariables|GetLastWaypoint) (.TargetLocation (Utilities|Struct|BreakCommandStruct (Utilities|Array|Get(acopy) _commandqueue _index))) (Variables|Default|GetPlayerController) 0))
    (LocalVariables|SetLastWaypoint (Utilities|Array|Get(acopy) (Variables|/Script/NavigationSystem.NavigationPath|GetPathPoints _returnvalue) (Utilities|Array|LastIndex (Variables|/Script/NavigationSystem.NavigationPath|GetPathPoints _returnvalue))))
    (Utilities|Array|RemoveIndex _returnarray (Utilities|Array|LastIndex _returnarray))
    (Utilities|Array|AppendArray (LocalVariables|GetReturnArray) (Variables|/Script/NavigationSystem.NavigationPath|GetPathPoints _returnvalue))
    (Utilities|Array|Add (Variables|Default|GetCommandDestinations) (LocalVariables|GetLastWaypoint)))
  (return (LocalVariables|GetReturnArray)))

(fn SelectFinalStartLocation
  (bind _queuepath (Variables|PartialPath|GetQueuePath))
  (if (Variables|Default|GetIsQueueEmpty)
    (return (Transformation|GetActorLocation (Variables|Default|GetControlledMember)))
    (else
      (return (select (== (Utilities|Array|Length _queuepath) 0) (Variables|Default|GetCurrentDestination) (Utilities|Array|Get(acopy) _queuepath (Utilities|Array|LastIndex _queuepath)))))))

(fn SetLinearSplinePoints
  (bind _spline (Variables|Default|GetSpline))
  (for _index (range 0 (Spline|GetNumberOfSplinePoints _spline))
    (Spline|SetSplinePointType _spline _index "Linear" true)))

(fn CalcSegmentCount
  (return (.ReturnValue (Math|Float|Division(WholeandRemainder) (Spline|GetSplineLength (Variables|Default|GetSpline)) (Variables|Default|GetWaypointSpacing)))))

(fn GenerateMeshes
  (params (SplinePoints :type Array%20of%20Vectors))
  (bind _returnvalue (CallFunction|CalcSegmentCount))
  (bind _spline (Variables|Default|GetSpline))
  (bind _splinemeshes (Variables|Default|GetSplineMeshes))
  (bind _spline_2 (Variables|Default|GetSpline))
  (if (> (Utilities|Array|Length SplinePoints) 0)
    (Spline|SetSplinePoints (Variables|Default|GetSpline) SplinePoints "World" true)
    (CallFunction|SetLinearSplinePoints)
    ;[1 1 1] Pre calculate MeshLength and SegmentCount
    (LocalVariables|SetMeshLength (/ (Spline|GetSplineLength (Variables|Default|GetSpline)) (Math|Conversions|ToFloat(Integer) _returnvalue)))
    (bind _output_get (LocalVariables|SetSegmentCount (- _returnvalue 1)))
    (Utilities|FlowControl|Sequence
      (:then_0
        ;[1 1 1] Spawn more meshes if needed
        (while (< (Utilities|Array|Length (Variables|Default|GetSplineMeshes)) (LocalVariables|GetSegmentCount))
          (bind _returnvalue_2 (AddComponent|AddSplineMeshComponent false))
          (Utilities|Array|Add (Variables|Default|GetSplineMeshes) _returnvalue_2)))
      (:then_1
        ;[1 1 1] Remove unneeded meshes.
        (while (> (Utilities|Array|Length (Variables|Default|GetSplineMeshes)) (LocalVariables|GetSegmentCount))
          (Components|DestroyComponent (Utilities|Array|Get(acopy) _splinemeshes))
          (Utilities|Array|RemoveIndex _splinemeshes)))
      (:then_2
        ;[1 1 1] Set mesh locations.
        (for _index (range 0 (LocalVariables|GetSegmentCount))
          (bind _output_get_2 (LocalVariables|SetIndex _index))
          (Utilities|IsValid (Utilities|Array|Get(acopy) (Variables|Default|GetSplineMeshes) _output_get_2)
            (:Is%20Valid
              (SplineMesh|SetStartandEnd (Utilities|Array|Get(acopy) (Variables|Default|GetSplineMeshes) _output_get_2) (Spline|GetLocationatDistanceAlongSpline _spline_2 (* (LocalVariables|GetIndex) (LocalVariables|GetMeshLength)) "Local") (* (Math|Vector|Normalize (Spline|GetTangentatDistanceAlongSpline _spline_2 (* (LocalVariables|GetIndex) (LocalVariables|GetMeshLength)) "Local") 0.0) (LocalVariables|GetMeshLength)) (Spline|GetLocationatDistanceAlongSpline _spline (* (+ (LocalVariables|GetIndex) 1) (LocalVariables|GetMeshLength)) "Local") (* (Math|Vector|Normalize (Spline|GetTangentatDistanceAlongSpline _spline (* (Math|Integer|SelectInt (+ (LocalVariables|GetIndex) 1) (LocalVariables|GetIndex) (>= _output_get (+ (LocalVariables|GetIndex) 1))) (LocalVariables|GetMeshLength)) "Local") 0.0) (LocalVariables|GetMeshLength)) true :!class /Script/Engine.SplineMeshComponent))))))
    (else
      (CallFunction|ClearSplineMeshes))))

(fn CalcPathtoCursor
  (bind _returnvalue (Class|NavigationSystemV1|FindPathtoLocationSynchronously (CallFunction|SelectFinalStartLocation) (.Location (Collision|BreakHitResult (.HitResult (Game|Player|GetHitResultUnderCursorbyChannel (Variables|Default|GetPlayerController) "TraceTypeQuery1" true)))) (Variables|Default|GetPlayerController) 0))
  (if (Class|NavigationPath|IsPartial _returnvalue)
    (return 0)
    (else
      (return (Variables|/Script/NavigationSystem.NavigationPath|GetPathPoints _returnvalue)))))

(fn UpdatePathChanges
  (params (ExistingPath :type Array%20of%20Vectors) (NewCalculation :type Array%20of%20Vectors))
  (bind _returnvalue (Utilities|Array|Identical ExistingPath NewCalculation))
  (if _returnvalue
    _
    (else
      (|SetBy-RefVar ExistingPath NewCalculation)))
  (return _returnvalue))

(fn ClearSplineMeshes
  (for _array_element (Variables|Default|GetSplineMeshes)
    (Components|DestroyComponent _array_element))
  (Utilities|Array|Clear (Variables|Default|GetSplineMeshes)))

(fn CalcCurrentPath
  (if (Variables|Default|GetIsQueueEmpty)
    (return 0)
    (else
      (bind _returnvalue (Class|NavigationSystemV1|FindPathtoLocationSynchronously (Transformation|GetActorLocation (Variables|Default|GetControlledMember)) (select (Utilities|IsValid (Variables|Default|GetTargetActor)) (Transformation|GetActorLocation) (Variables|Default|GetCurrentDestination)) (Variables|Default|GetPlayerController) 0))
      (return (Variables|/Script/NavigationSystem.NavigationPath|GetPathPoints _returnvalue)))))