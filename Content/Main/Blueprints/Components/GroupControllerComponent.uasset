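; Actor component that manages a size-capped group of members for its owner and tracks one selected member.
; Recruit and remove send requests to the target or its group member component, while separate join and left events update the member list.
; A departing selected member clears the selection, and Validate checks whether a target's member component reports this owner.
; On EndPlay it notifies every member that the owner has ended.
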(event Custom|EventRecruitToGroup
  (params (RecruitTarget :type Group%20Member%20Component%20Object%20Reference))
  (Default|EventRequestGroupJoin RecruitTarget self))

(event Custom|EventRemoveFromGroup
  (params (RemoveTarget :type Actor%20Object%20Reference))
  (bind _component (Class|IGroupMemberComponent|GetGroupMemberComponent(Message) RemoveTarget))
  (Default|EventLeaveGroup _component (Components|GetOwner self)))

(event Custom|EventSelectMember
  (params (PartyMemberIndex :type Integer))
  (bind _output_get (Variables|Default|SetSelectedMemberIndex PartyMemberIndex))
  (Variables|Default|SetSelectedMember (Utilities|Array|Get(acopy) (Variables|Default|GetGroupMembers) _output_get)))

(event Custom|EventClearSelection
  (Variables|Default|SetSelectedMember 0))

(event Custom|EventMemberJoin
  (params (JoiningMember :type Actor%20Object%20Reference))
  (if (not (CallFunction|IsGroupFull))
    (Utilities|Array|AddUnique (Variables|Default|GetGroupMembers) JoiningMember)))

(event Custom|EventMemberLeft
  (params (LeavingMember :type Actor%20Object%20Reference))
  (if (== LeavingMember (Variables|Default|GetSelectedMember))
    (CallFunction|EventClearSelection))
  (Utilities|Array|RemoveItem (Variables|Default|GetGroupMembers) LeavingMember))

(event EventEndPlay
  (params (EndPlayReason :type EEndPlayReason%20Enum :default "Destroyed"))
  (for _array_element (Variables|Default|GetGroupMembers)
    (bind _component (Class|IGroupMemberComponent|GetGroupMemberComponent(Message) _array_element))
    (Default|EventOwnerEnded _component (Components|GetOwner self))))

(fn IsGroupFull
  (return (not (< (Utilities|Array|Length (Variables|Default|GetGroupMembers)) (Variables|Default|GetGroupSize)))))

(fn Validate
  (params (RequestTarget :type Actor%20Object%20Reference))
  (bind _component (Class|IGroupMemberComponent|GetGroupMemberComponent(Message) RequestTarget))
  (return (== (Default|GetOuterOwner _component) (Components|GetOwner self))))

(fn GetSelectedMember
  (return (Variables|Default|GetSelectedMember)))

(fn GetMember
  (params (Index :type Integer))
  (return (Utilities|Array|Get(acopy) (Variables|Default|GetGroupMembers) Index)))