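; Actor component that lets its owning actor join and leave a group led by an actor with a GroupControllerComponent.
; Joining, allowed only when not already grouped, makes the group owner the member's Owner and notifies the controller.
; Leaving, accepted only from that group owner, notifies the controller and sets Owner back to the member's AI controller.
; An owner-ended event just clears the stored group owner.
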(event Custom|EventRequestGroupJoin
  (params (GroupControllerComponent :type Group%20Controller%20Component%20Object%20Reference))
  (bind _self self)
  (bind _returnvalue (Components|GetOwner _self))
  (if (not (Utilities|IsValid (Variables|Default|GetGroupOwnerActor)))
    (bind _output_get (Variables|Default|SetGroupOwnerActor (Components|GetOwner GroupControllerComponent)))
    (Actor|SetOwner _returnvalue _output_get)
    (Default|EventMemberJoin GroupControllerComponent _returnvalue)))

(event Custom|EventOwnerEnded
  (params (Instigator :type Actor%20Object%20Reference))
  (if (== Instigator (Variables|Default|GetGroupOwnerActor))
    (Variables|Default|SetGroupOwnerActor 0)))

(event Custom|EventLeaveGroup
  (params (Instigator :type Actor%20Object%20Reference))
  (bind _self self)
  (bind _returnvalue (Components|GetOwner _self))
  (if (== Instigator (Variables|Default|GetGroupOwnerActor))
    (Variables|Default|SetGroupOwnerActor 0)
    (bind _component (Class|IGroupControllerComponent|GetGroupControllerComponent(Message) Instigator))
    (Default|EventMemberLeft _component (Components|GetOwner self))
    (Actor|SetOwner _returnvalue (AI|GetAIController _returnvalue))))

(fn GetOuterOwner
  (return (Components|GetOwner (Components|GetOwner))))