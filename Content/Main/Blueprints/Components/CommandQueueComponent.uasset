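; Component that gives its owning pawn a capped queue of ability commands, executed one at a time.
; Each command spawns its ability actor at the owner and activates it on the target; completion removes the head and starts the next.
; The ability's ClearListOnCommand default, inverted by the modifier key, decides whether a new command clears the queue and destroys the running ability.
; Cancelling only removes the queue entry, without notifying or stopping the running ability.
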(event Custom|EventGiveCommand
  (params (Command :type Command%20Struct%20Structure) (ModifierPressed :type Boolean))
  (CallFunction|ClearQueueifNeeded Command ModifierPressed)
  (bind _success (CallFunction|AddtoQueue Command))
  (if _success
    (if (not (Variables|Default|GetExecuting))
      (Default|CallQueueChanged)
      (CallFunction|ExecuteNextCommand))))

(event Custom|EventCancelCommand
  (params (Index :type Integer))
  (CallFunction|RemovefromQueue Index))

(event Custom|EventCommandCompleted
  (Utilities|Array|RemoveIndex (Variables|Default|GetExecutionQueue))
  (Default|CallQueueChanged)
  (CallFunction|ExecuteNextCommand))

(event EventTick
  (params (DeltaSeconds :type Float%20%28single-precision%29)))

(event EventBeginPlay
  (bind _aspawn (Utilities|Casting|CastToPawn (Components|GetOwner)))
  (Variables|Default|SetOwnerPawn _aspawn))

(fn IsQueueEmpty
  (return (== (Utilities|Array|Length (Variables|Default|GetExecutionQueue)) 0)))

(fn IsQueueFull
  (return (>= (Utilities|Array|Length (Variables|Default|GetExecutionQueue)) (Variables|Default|GetQueueSize))))

(fn ExecuteNextCommand
  (bind _ownerpawn (Variables|Default|GetOwnerPawn))
  (bind (_nextcommand _success) (CallFunction|GetNextfromQueue))
  (if _success
    (bind _returnvalue (Game|SpawnActorfromClass (.Ability (Utilities|Struct|BreakCommandStruct _nextcommand)) (Math|Transform|MakeTransform (Transformation|GetActorLocation (Components|GetOwner)) "0, 0, 0" "1,1,1") "AlwaysSpawn" _ownerpawn _ownerpawn))
    (bind _output_get (Variables|Default|SetCurrentAbility _returnvalue))
    (Default|ActivateAbility _output_get (.TargetActor (Utilities|Struct|BreakCommandStruct _nextcommand)) (.TargetLocation (Utilities|Struct|BreakCommandStruct _nextcommand)))
    (Variables|Default|SetExecuting true)
    (else
      (Variables|Default|SetExecuting false))))

(fn RemovefromQueue
  (params (RemovedIndex :type Integer))
  (Utilities|Array|RemoveIndex (Variables|Default|GetExecutionQueue) RemovedIndex))

(fn AddtoQueue
  (params (NewCommand :type Command%20Struct%20Structure%20%28by%20ref%29))
  (if (not (CallFunction|IsQueueFull))
    (Utilities|Array|Add (Variables|Default|GetExecutionQueue) NewCommand)
    (return true)
    (else
      (return false))))

(fn GetNextfromQueue
  (if (not (CallFunction|IsQueueEmpty))
    (return (Utilities|Array|Get(acopy) (Variables|Default|GetExecutionQueue)) true)
    (else
      (return "" false))))

(fn ClearQueueifNeeded
  (params (Command :type Command%20Struct%20Structure) (ModifierPressed :type Boolean))
  (bind _ability (Utilities|Struct|BreakCommandStruct Command))
  (bind _currentability (Variables|Default|GetCurrentAbility))
  (bind _clearlistoncommand (Utilities|GetClassDefaults _ability))
  (if (select ModifierPressed (not _clearlistoncommand) _clearlistoncommand)
    (Utilities|Array|Clear (Variables|Default|GetExecutionQueue))
    (Utilities|IsValid _currentability
      (:Is%20Valid
        (Actor|DestroyActor _currentability))
      (:Is%20Not%20Valid
        _))
    (Variables|Default|SetExecuting false)))