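; Actor component that tracks talent unlock states across equipped talent trees and grants or removes their abilities.
; Lock and unlock events resolve tree and talent indices through TalentTreeData and the talent tree DataTable, then update that tree's state array.
; On success, the talent's ability class from TalentsTable is added to or removed from the owner's AbilityContainer.
; SetTalentState ignores NewUnlockedValue and always writes true, so locking leaves talents unlocked.
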(event Custom|EventLockTalent
  (params (TalentTreeName :type Name) (TalentName :type Name))
  (bind _success (Basics|SetTalentState TalentTreeName TalentName false))
  (if _success
    (AbilityContainer|RemoveAbilityfromContainer TalentName)))

(event Custom|EventUnlockTalent
  (params (TalentTreeName :type Name) (TalentName :type Name))
  (bind _success (Basics|SetTalentState TalentTreeName TalentName true))
  (if _success
    (AbilityContainer|AddAbilitytoContainer TalentName)))

(event EventBeginPlay
  (bind _component (Class|IAbilityContainer|GetAbilityContainerComponent(Message) (Components|GetOwner)))
  (Variables|AbilityContainer|SetAbilityContainer _component))

(fn CheckTalentState
  (params (TalentTreeName :type Name) (TalentName :type Name))
  (bind (_treeindex _found) (Basics|FindEquippedTree TalentTreeName))
  (if _found
    (bind (_talentindex _found_2) (Basics|FindTalentinTree TalentTreeName TalentName))
    (if _found_2
      (return (Utilities|Array|Get(acopy) (.talentunlockstatearray (Utilities|Array|Get(acopy) (Variables|Default|GetTalentTreeData) _treeindex)) _talentindex))
      (else
        (return false)))
    (else
      (return false))))

(fn FindTalentinTree
  (params (TalentTreeRowName :type Name) (TalentName :type Name))
  (bind _returnvalue (Utilities|GetDataTableRow "/Game/Main/DataTables/TalentTreeTable.TalentTreeTable" TalentTreeRowName)
    (:then
      (return (Utilities|Array|FindItem (.talentrownames _returnvalue) TalentName) (>= (Utilities|Array|FindItem (.talentrownames _returnvalue) TalentName) 0)))
    (:RowNotFound
      (return -1 false))))

(fn FindEquippedTree
  (params (TalentTreeName :type Name))
  (bind (_array_element _array_index) (Utilities|Array|ForEachLoopwithBreak (Variables|Default|GetTalentTreeData) :!label _label)
    (:LoopBody
      (if (Utilities|Name|Equal(Name) TalentTreeName (.talenttreerowname _array_element))
        (LocalVariables|SetIndex _array_index)
        (goto _label Break)))
    (:Completed
      (return (LocalVariables|GetIndex) (>= (LocalVariables|GetIndex) 0)))))

(fn CheckTalentHasAbility
  (params (TalentRowName :type Name))
  (bind _returnvalue (Utilities|GetDataTableRow "/Game/Main/DataTables/TalentsTable.TalentsTable" TalentRowName)
    (:then
      (return (Utilities|IsValidClass (.abilitiy _returnvalue))))
    (:RowNotFound
      (return false))))

(fn SetTalentState
  (params (TalentTreeName :type Name) (TalentName :type Name) (NewUnlockedValue :type Boolean))
  (bind (_treeindex _found) (Basics|FindEquippedTree TalentTreeName))
  (if _found
    (bind (_talentindex _found_2) (Basics|FindTalentinTree TalentTreeName TalentName))
    (if _found_2
      (Utilities|Array|SetArrayElem (.talentunlockstatearray (Utilities|Array|Get(acopy) (Variables|Default|GetTalentTreeData) _treeindex)) _talentindex true)
      (return true)
      (else
        _)))
  (return false))

(fn AddAbilitytoContainer
  (params (TalentName :type Name))
  (bind _abilitycontainer (Variables|AbilityContainer|GetAbilityContainer))
  (bind _return (Basics|CheckTalentHasAbility TalentName))
  (if (and _return (Utilities|IsValid _abilitycontainer))
    (bind _returnvalue (Utilities|GetDataTableRow "/Game/Main/DataTables/TalentsTable.TalentsTable" TalentName)
      (:then
        (Default|EventAddAbility _abilitycontainer (.abilitiy _returnvalue))))))

(fn RemoveAbilityfromContainer
  (params (TalentName :type Name))
  (bind _abilitycontainer (Variables|AbilityContainer|GetAbilityContainer))
  (bind _return (Basics|CheckTalentHasAbility TalentName))
  (if (and _return (Utilities|IsValid _abilitycontainer))
    (bind _returnvalue (Utilities|GetDataTableRow "/Game/Main/DataTables/TalentsTable.TalentsTable" TalentName)
      (:then
        (Default|EventRemoveAbility _abilitycontainer (.abilitiy _returnvalue))))))