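; AbilityContainerComponent is a component that stores a list of ability classes for its owner.
; Add and remove events forward to helper functions that insert a class only if it is not already present or remove the first match.
; GetAbility returns the entry at a given index without a bounds check.
; The EventAssessUsefulness event is an empty stub.
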(event Custom|EventAddAbility
  (params (NewAbilityClass :type Ability%20Base%20Class%20Reference))
  (CallFunction|AddtoContainer NewAbilityClass))

(event Custom|EventRemoveAbility
  (params (AbilityClass :type Ability%20Base%20Class%20Reference))
  (CallFunction|RemovefromContainer AbilityClass))

(event Custom|EventAssessUsefulness)

(fn AddtoContainer
  (params (NewAbilityClass :type Ability%20Base%20Class%20Reference))
  (bind _array_element (Utilities|Array|ForEachLoopwithBreak (Variables|Default|GetAbilities) :!label _label)
    (:LoopBody
      (if (== _array_element NewAbilityClass)
        (LocalVariables|SetAbilityAlreadyExist true)
        (goto _label Break)))
    (:Completed
      (if (not (LocalVariables|GetAbilityAlreadyExist))
        (Utilities|Array|AddUnique (Variables|Default|GetAbilities) NewAbilityClass)))))

(fn RemovefromContainer
  (params (AbilityClass :type Ability%20Base%20Class%20Reference))
  (bind _array_element (Utilities|Array|ForEachLoopwithBreak (Variables|Default|GetAbilities) :!label _label)
    (:LoopBody
      (if (== _array_element AbilityClass)
        (Utilities|Array|RemoveItem (Variables|Default|GetAbilities) _array_element)
        (goto _label Break)))))

(fn GetAbility
  (params (Index :type Integer))
  (return (Utilities|Array|Get(acopy) (Variables|Default|GetAbilities) Index)))